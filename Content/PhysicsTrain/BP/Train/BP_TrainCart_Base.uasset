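; BP_TrainCart_Base is a physics-driven train cart that follows rail splines, with simple mouse-look control.
; Each tick, a downward box trace at two carriage sockets caches the rail fragment spline beneath each.
; A damped spring force, projected perpendicular to the track, pulls each socket toward its spline while leaving forward motion free.
; A damped spring torque around the forward axis keeps the body's roll level.
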(event EventTick
  (params (DeltaSeconds :type Float%20%28single-precision%29))
  (Utilities|FlowControl|Sequence
    (:then_0
      ;[1 1 1] simplest look control
      (Pawn|Input|AddControllerYawInput (Class|Actor|GetInputAxisKeyValue))
      (Pawn|Input|AddControllerPitchInput (* (Class|Actor|GetInputAxisKeyValue) -1.0)))
    (:then_1
      (CallFunction|ProcessCart "VisualCarriage_1")
      (CallFunction|ProcessCart "VisualCarriage_2")
      (CallFunction|ControlRotation))))

(fn ConstructionScript)

(fn ProcessCart
  (params (CarriageSocket :type Name))
  ;[1 1 1] Prepair
  (LocalVariables|SetCurrentLocation (Transformation|GetSocketLocation (Variables|Default|GetTrainBody) CarriageSocket))
  (CallFunction|FindRels (LocalVariables|GetCurrentLocation) CarriageSocket)
  (bind _output_get (LocalVariables|SetTestSplineComponent (.spline (.Value (Utilities|Map|Find (Variables|Default|GetSplineComponentsBysocket) CarriageSocket)))))
  (Utilities|IsValid _output_get
    (:Is%20Valid
      (LocalVariables|SetProjectedToSpline (Class|SplineComponent|FindTransformClosesttoWorldLocation (LocalVariables|GetTestSplineComponent) (LocalVariables|GetCurrentLocation) "World" false))
      ;[1 1 1] apply handle forces
      (bind _returnvalue (Class|PrimitiveComponent|GetPhysicsLinearVelocityatPoint (Variables|Default|GetTrainBody) (LocalVariables|GetCurrentLocation) CarriageSocket))
      (Class|PrimitiveComponent|AddForceatLocation (Variables|Default|GetTrainBody) (Math|Vector|ProjectVectorontoPlane (+ (* _returnvalue (* -1.0 (Variables|Default|GetDamping))) (* (- (.location (LocalVariables|GetProjectedToSpline)) (+ (LocalVariables|GetCurrentLocation) (LocalVariables|GetForceCorrectionOffset))) (Variables|Default|GetStiffness))) (Math|Vector|GetForwardVector (.rotation (LocalVariables|GetProjectedToSpline)))) (LocalVariables|GetCurrentLocation) "None"))))

(fn FindRels
  (params (Start :type Vector) (Socket :type Name%20%28by%20ref%29))
  (bind _splinecomponentsbysocket (Variables|Default|GetSplineComponentsBysocket))
  (bind (_value _returnvalue) (Utilities|Map|Find _splinecomponentsbysocket Socket))
  (LocalVariables|SetIsSuccess false)
  (bind _outhits (Class|KismetSystemLibrary|BoxTraceMultiforObjects Start (+ Start "0.000000,0.000000,-50.000000") "10.000000,10.000000,10.000000" "0, 0, 0" (Utilities|Array|MakeArray "ObjectTypeQuery2") false 0 "ForOneFrame" true))
  (bind _array_element (Utilities|Array|ForEachLoopwithBreak _outhits :!label _label)
    (:LoopBody
      (bind _asbp_rails_fragment_base (Utilities|Casting|CastToBP_RailsFragmentBase (.hitactor _array_element)))
      (bind _output_get (LocalVariables|SetRailsLocal _asbp_rails_fragment_base))
      (if (and (== (.rail _value) _output_get) _returnvalue)
        _
        (else
          (Utilities|Map|Add (Variables|Default|GetSplineComponentsBysocket) Socket (Utilities|Struct|MakeS_FindRailStruct (LocalVariables|GetRailsLocal) (Default|GetSplineComponent (LocalVariables|GetRailsLocal) self)))))
      (LocalVariables|SetIsSuccess true)
      (goto _label Break))
    (:Completed
      (if (not (LocalVariables|GetIsSuccess))
        (Utilities|Map|Add :TargetMap (Variables|Default|GetSplineComponentsBysocket) :Key Socket)))))

(fn ControlRotation
  (LocalVariables|SetTrainRotation (Transformation|GetWorldRotation (Variables|Default|GetTrainBody)))
  (Class|PrimitiveComponent|AddTorqueinDegrees (Variables|Default|GetTrainBody) (+ (* (Math|Vector|ProjectVectorontoVector (Physics|GetPhysicsAngularVelocityinDegrees (Variables|Default|GetTrainBody) "None") (Math|Vector|GetForwardVector (LocalVariables|GetTrainRotation))) (* (Variables|Default|GetRotationDamping) -1.0)) (* (Math|Vector|GetForwardVector (LocalVariables|GetTrainRotation)) (* (Math|Float|Sign(Float) (.Z (Math|Vector|BreakVector (Math|Vector|GetRightVector (LocalVariables|GetTrainRotation))))) (Class|KismetMathLibrary|DegAcos (Math|Vector|DotProduct (Math|Vector|GetRightVector (LocalVariables|GetTrainRotation)) (Math|Vector|GetRightVector (Math|Rotator|MakeRotator 0.0 0.0 (.yaw (LocalVariables|GetTrainRotation)))))) (Variables|Default|GetRotationStiffness) -1.0))) "None" true))