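; BP_RailsTest_Switch is a rail switch for the physics train that chooses between a left and a right spline.
; GetSplineComponent returns the left or right spline when the passed train overlaps that side's enter component, checking left first.
; Otherwise the boolean State decides: true gives right, false gives left.
; State resets to false on BeginPlay, and nothing in these graphs toggles it.
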(event EventBeginPlay
  (Variables|Default|SetState false))

(fn ConstructionScript)

(fn GetSplineComponent
  (params (Self%20triain :type BP%20Train%20Cart%20Base%20Object%20Reference))
  (if (Utilities|Array|ContainsItem (Collision|GetOverlappingActors (Variables|Default|GetLeftEnter) 0 :!class /Script/Engine.PrimitiveComponent) Self%20triain)
    (return (Variables|Default|GetSpline_L))
    (elif (Utilities|Array|ContainsItem (Collision|GetOverlappingActors (Variables|Default|GetRightEnter) 0 :!class /Script/Engine.PrimitiveComponent) Self%20triain)
      (return (Variables|Default|GetSpline_R))
      (elif (Variables|Default|GetState)
        (return (Variables|Default|GetSpline_R))
        (else
          (return (Variables|Default|GetSpline_L)))))))