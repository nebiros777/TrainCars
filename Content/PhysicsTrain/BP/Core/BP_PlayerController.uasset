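; Player controller for the physics train, letting the player drive a train cart.
; On BeginPlay it finds a BP_TrainCart_Base actor in the level, stores it and possesses it.
; The MoveForward axis feeds the cart's engine power, and pressing or releasing Brake toggles its brakes, leaving the response to the cart itself.
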(event EventBeginPlay
  ;[1 1 1] Possess our cart on a map
  (bind _returnvalue (Actor|GetActorOfClass "/Game/PhysicsTrain/BP/Train/BP_TrainCart_Base.BP_TrainCart_Base_C"))
  (bind _asbp_train_cart_base (Utilities|Casting|CastToBP_TrainCart_Base _returnvalue))
  (bind _output_get (Variables|Default|SetAs%20BP%20Train%20Cart%20Base _asbp_train_cart_base))
  (Pawn|Possess _output_get))

(event EventTick
  (params (DeltaSeconds :type Float%20%28single-precision%29)))

(event Input|ActionEvents|InputActionBrake
  (params (Key :type Key%20Structure :default "None"))
  (bind _as_bp_train_cart_base (Variables|Default|GetAs%20BP%20Train%20Cart%20Base))
  ;[1 1 1] Input
  (:Pressed
    (Default|ManageBrakes _as_bp_train_cart_base true))
  (:Released
    (Default|ManageBrakes _as_bp_train_cart_base false)))

(event Input|AxisEvents|InputAxisMoveForward
  (params (AxisValue :type Float%20%28single-precision%29))
  ;[1 1 1] Input
  (Default|ManageEnginePower (Variables|Default|GetAs%20BP%20Train%20Cart%20Base) AxisValue))

(fn ConstructionScript)